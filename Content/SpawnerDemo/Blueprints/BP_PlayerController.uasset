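; Player controller for the spawner demo that creates the local HUD, adds the input mapping and handles map hotkeys.
; Input actions reload the level, return to MainMap or player start through server events, or toggle the HUD map.
; Outside MainMap, the authority saves pawn transform to the GameMode's ServerArchive on UnPossess and restores it on BeginPlay.
; A gold counter updates the HUD locally and through its OnRep.
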(event `self.ReceiveBeginPlay`
  (bind _returnvalue (subsystem `EnhancedInputLocalPlayerSubsystem`))
  (bind _returnvalue_2 (`GameplayStatics.GetCurrentLevelName` true))
  (set `self.MapName` _returnvalue_2)
  (`self.SetPawnPosition`)
  (if (`self.IsLocalPlayerController`)
    (bind _returnvalue_3 (`|CreateWidget` "/Game/SpawnerDemo/Blueprints/W_HUD.W_HUD_C"))
    (bind _output_get (set `self.HUDWidget` _returnvalue_3))
    (`UserWidget.AddToPlayerScreen` _output_get 0)
    (`/Engine/EditorBlueprintResources/StandardMacros.IsValid` _returnvalue
      (:`Is Valid`
        (`EnhancedInputSubsystemInterface.AddMappingContext` _returnvalue "/Game/SpawnerDemo/Input/IMC_Default.IMC_Default" 0 (struct))))))

(event `self.ReceiveUnPossess`
  (params (UnpossessedPawn :type "Pawn Object Reference"))
  (`self.SavePawnPosition` UnpossessedPawn))

(event `Server_OpenLevel`
  (`self.ServerTravel` (`self.MapName`)))

(event `EnhancedInput|/Game/SpawnerDemo/Input/IA_Reload`
  (params (ActionValue :type Boolean) (ElapsedSeconds :type "Float (double-precision)") (TriggeredSeconds :type "Float (double-precision)") (InputAction :type "InputAction Object Reference" :default "/Game/SpawnerDemo/Input/IA_Reload.IA_Reload"))
  (:`Triggered`
    (`self.Server_OpenLevel`)))

(event `EnhancedInput|/Game/SpawnerDemo/Input/IA_ReturnToStart`
  (params (ActionValue :type Boolean) (ElapsedSeconds :type "Float (double-precision)") (TriggeredSeconds :type "Float (double-precision)") (InputAction :type "InputAction Object Reference" :default "/Game/SpawnerDemo/Input/IA_ReturnToStart.IA_ReturnToStart"))
  (:`Triggered`
    (if (not (`self.IsInMainMap`))
      (`self.Server_ReturnToStart`))))

(event `Server_ReturnToStart`
  (`self.ReturnToStart`))

(event `EnhancedInput|/Game/SpawnerDemo/Input/IA_MainMap`
  (params (ActionValue :type Boolean) (ElapsedSeconds :type "Float (double-precision)") (TriggeredSeconds :type "Float (double-precision)") (InputAction :type "InputAction Object Reference" :default "/Game/SpawnerDemo/Input/IA_MainMap.IA_MainMap"))
  (:`Triggered`
    (if (not (`self.IsInMainMap`))
      (`self.Server_MainMap`))))

(event `Server_MainMap`
  (`self.ServerTravel` "MainMap"))

(event `EnhancedInput|/Game/SpawnerDemo/Input/IA_Map`
  (params (ActionValue :type Boolean) (ElapsedSeconds :type "Float (double-precision)") (TriggeredSeconds :type "Float (double-precision)") (InputAction :type "InputAction Object Reference" :default "/Game/SpawnerDemo/Input/IA_Map.IA_Map"))
  (:`Triggered`
    (if (not (`self.IsInMainMap`))
      (bind _hudwidget (`self.HUDWidget`)
        (:`then`
          (`/Game/SpawnerDemo/Blueprints/W_HUD.SwitchMap` _hudwidget))
        (:`else`)))))

(fn `AddGoldQuantity`
  (params (InQuantity :type Integer))
  (set `self.GoldCount` (+ (`self.GoldCount`) InQuantity))
  (if (`self.IsLocalController`)
    (bind _hudwidget (`self.HUDWidget`)
      (:`then`
        (`/Game/SpawnerDemo/Blueprints/W_HUD.SetGoldCount` _hudwidget (`self.GoldCount`)))
      (:`else`))))

(fn `IsInMainMap`
  (returns (bReturnValue :type Boolean))
  (return (`KismetStringLibrary.EqualEqual_StrStr` (`self.MapName`) "MainMap")))

(fn `OnRep_GoldCount`
  (bind _hudwidget (`self.HUDWidget`)
    (:`then`
      (`/Game/SpawnerDemo/Blueprints/W_HUD.SetGoldCount` _hudwidget (`self.GoldCount`)))
    (:`else`)))

(fn `ReturnToStart`
  (bind _returnvalue (`self.K2_GetPawn`))
  (bind (_returnvalue_location _returnvalue_rotation) (`KismetMathLibrary.BreakTransform` (`self.GetTransform` (`GameModeBase.K2_FindPlayerStart` (`GameplayStatics.GetGameMode`) self ""))))
  (`/Engine/EditorBlueprintResources/StandardMacros.IsValid` _returnvalue
    (:`Is Valid`
      (`self.K2_SetActorTransform` _returnvalue (`KismetMathLibrary.MakeTransform` _returnvalue_location _returnvalue_rotation (`self.GetActorScale3D` _returnvalue)) false false))))

(fn `SavePawnPosition`
  (params (InPawn :type "Pawn Object Reference"))
  (locals (OwnerPawn :type "Pawn Object Reference"))
  (`/Engine/EditorBlueprintResources/ActorMacros.Switch Has Authority`
    (:`Authority`
      (if (not (`self.IsInMainMap`))
        (bind _asbp_game_mode (cast `/Game/SpawnerDemo/Blueprints/BP_GameMode` (`GameplayStatics.GetGameMode`)))
        (bind _serverarchive (`/Game/SpawnerDemo/Blueprints/BP_GameMode.ServerArchive` _asbp_game_mode)
          (:`then`
            (set `/Game/SpawnerDemo/SaveGame/SG_ServerArchive.PlayerTransform` (`self.GetTransform` (`local.InPawn`)) _serverarchive))
          (:`else`))))))

(fn `ServerTravel`
  (params (NewMapName :type String))
  (`KismetSystemLibrary.ExecuteConsoleCommand` (`KismetStringLibrary.Concat_StrStr` "ServerTravel " NewMapName) null))

(fn `SetPawnPosition`
  (locals (OwnerPawn :type "Pawn Object Reference"))
  (`/Engine/EditorBlueprintResources/ActorMacros.Switch Has Authority`
    (:`Authority`
      (if (not (`self.IsInMainMap`))
        (bind _output_get (set `local.OwnerPawn` (`self.K2_GetPawn`)))
        (`/Engine/EditorBlueprintResources/StandardMacros.IsValid` _output_get
          (:`Is Valid`
            (bind _asbp_game_mode (cast `/Game/SpawnerDemo/Blueprints/BP_GameMode` (`GameplayStatics.GetGameMode`)))
            (bind _serverarchive (`/Game/SpawnerDemo/Blueprints/BP_GameMode.ServerArchive` _asbp_game_mode)
              (:`then`
                (bind _playertransform (`/Game/SpawnerDemo/SaveGame/SG_ServerArchive.PlayerTransform` _serverarchive))
                (if (not (`KismetMathLibrary.Vector_IsNearlyZero` (.location _playertransform)))
                  (`self.K2_SetActorTransform` (`local.OwnerPawn`) _playertransform false false)
                  (`self.SetControlRotation` (.rotation _playertransform))))
              (:`else`))))))))

(fn `UserConstructionScript`)