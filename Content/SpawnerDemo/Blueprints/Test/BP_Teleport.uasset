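; BP_Teleport is a level-transition pad that moves players to TargetLevel when a player-controlled pawn overlaps its Trigger.
; In standalone it opens the level by object reference, otherwise it runs a ServerTravel console command using the package path split from the level's soft object path.
; The construction script tints the Plate blue through its Color material parameter.
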(event `self.Trigger.OnComponentBeginOverlap`
  (params (OverlappedComponent :type "PrimitiveComponent Object Reference") (OtherActor :type "Actor Object Reference") (OtherComp :type "PrimitiveComponent Object Reference") (OtherBodyIndex :type Integer) (bFromSweep :type Boolean) (SweepResult :type "HitResult Structure (by ref)"))
  (bind _returnvalue_pathstring (`KismetSystemLibrary.BreakSoftObjectPath` (`KismetSystemLibrary.Conv_SoftObjRefToSoftObjPath` (`self.TargetLevel`))))
  (bind _aspawn (cast `Pawn` OtherActor))
  (if (`Pawn.IsPlayerControlled` _aspawn)
    (if (`KismetSystemLibrary.IsStandalone`)
      (`GameplayStatics.OpenLevelBySoftObjectPtr` (`self.TargetLevel`))
      (else
        (`KismetSystemLibrary.ExecuteConsoleCommand` (`KismetStringLibrary.Concat_StrStr` "ServerTravel " (`KismetStringLibrary.Split` _returnvalue_pathstring ".")) null)))))

(fn `UserConstructionScript`
  (`MeshComponent.SetColorParameterValueOnMaterials` (`self.Plate`) "Color" (struct :`B` 1.0 :`A` 1.0)))