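; Spawnable tree entity for the SpawnerDemo that ages over time and dies when attacked or too old.
; InitEntity takes an EAS_Tree attribute set for its color, and AgeTime adds elapsed age to the initial age to drive the material's AgeRatio.
; Color and AgeRatio use RepNotifies to update materials on clients.
; Both death causes share one path: multicast physics simulation, then delayed destruction.
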(event `FPSpawnerEntityInterface.InitEntity`
  (params (EntityHandle :type "FPSpawnerEntityHandle Structure (by ref)") (AttributeSet :type "FPSpawnerEntityAttributeSet Object Reference"))
  (bind _aseas_tree (cast `/Game/SpawnerDemo/Data/AttributeSet/EAS_Tree` AttributeSet))
  (bind _output_get (set `self.AttributeSet` _aseas_tree))
  (bind _output_get_2 (set `self.Color` (`KismetMathLibrary.MakeVector` (`/Game/SpawnerDemo/Data/AttributeSet/EAS_Tree.Color_R` _output_get) (`/Game/SpawnerDemo/Data/AttributeSet/EAS_Tree.Color_G` _output_get) (`/Game/SpawnerDemo/Data/AttributeSet/EAS_Tree.Color_B` _output_get))))
  (`MeshComponent.SetVectorParameterValueOnMaterials` (`self.Tree`) "Color" _output_get_2))

(event `/Game/SpawnerDemo/Blueprints/Projectile/BPI_Projectile.OnAttack`
  (params (Owner :type "Actor Object Reference"))
  (if (not (`self.bDeath`))
    (set `self.bDeath` true :!label _label)
    (`self.NetMulticast_SetSimulatePhysics`)
    (`KismetSystemLibrary.Delay` 4.0)
    (`self.K2_DestroyActor`)))

(event `FPSpawnerEntityInterface.ReceiveAgeTime`
  (params (AgeTime :type "Float (single-precision)"))
  (if (not (`self.bDeath`))
    (bind _output_get (set `self.AgeRatio` (+ (/ AgeTime 50.0) (`/Game/SpawnerDemo/Data/AttributeSet/EAS_Tree.InitialAge` (`self.AttributeSet`)))))
    (if (> _output_get 1.1)
      (goto _label)
      (else
        (`MeshComponent.SetScalarParameterValueOnMaterials` (`self.Tree`) "AgeRatio" (`self.AgeRatio`))))))

(event `NetMulticast_SetSimulatePhysics`
  (`PrimitiveComponent.SetSimulatePhysics` (`self.Tree`) true))

(fn `OnRep_AgeRatio`
  (`MeshComponent.SetScalarParameterValueOnMaterials` (`self.Tree`) "AgeRatio" (`self.AgeRatio`)))

(fn `OnRep_Color`
  (`MeshComponent.SetVectorParameterValueOnMaterials` (`self.Tree`) "Color" (`self.Color`)))

(fn `UserConstructionScript`)