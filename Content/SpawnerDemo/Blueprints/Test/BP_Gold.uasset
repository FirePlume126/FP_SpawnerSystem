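; BP_Gold is a gold pickup that grants its quantity to the player who overlaps it.
; InitEntity reads Quantity from an attribute set and shows it on two text renders, destroying the actor if it is not positive.
; On server authority, sphere overlap by a player character adds the gold to its player controller and destroys the pickup.
; Tick spins the sphere by a fixed yaw each frame, independent of delta time.
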(event `self.ReceiveTick`
  (params (DeltaSeconds :type "Float (single-precision)"))
  (`SceneComponent.K2_AddWorldRotation` (`self.SphereComp`) (struct :`Yaw` 4.0) false false))

(event `FPSpawnerEntityInterface.InitEntity`
  (params (EntityHandle :type "FPSpawnerEntityHandle Structure (by ref)") (AttributeSet :type "FPSpawnerEntityAttributeSet Object Reference"))
  (bind _output_get (set `self.Quantity` (`FPSpawnerEntityAttributeSet.K2_GetAttribute` AttributeSet "Quantity")))
  (if (> _output_get 0)
    (`TextRenderComponent.K2_SetText` (`self.TextRender1`) (`KismetTextLibrary.Conv_IntToText` (`self.Quantity`)))
    (`TextRenderComponent.K2_SetText` (`self.TextRender`) (`KismetTextLibrary.Conv_IntToText` (`self.Quantity`)))
    (else
      (`self.K2_DestroyActor`))))

(event `self.SphereComp.OnComponentBeginOverlap`
  (params (OverlappedComponent :type "PrimitiveComponent Object Reference") (OtherActor :type "Actor Object Reference") (OtherComp :type "PrimitiveComponent Object Reference") (OtherBodyIndex :type Integer) (bFromSweep :type Boolean) (SweepResult :type "HitResult Structure (by ref)"))
  (`/Engine/EditorBlueprintResources/ActorMacros.Switch Has Authority`
    (:`Authority`
      (bind _asbp_player_character (cast `/Game/SpawnerDemo/Blueprints/BP_PlayerCharacter` OtherActor))
      (bind _asbp_player_controller (cast `/Game/SpawnerDemo/Blueprints/BP_PlayerController` (`Pawn.GetController` _asbp_player_character)))
      (`/Game/SpawnerDemo/Blueprints/BP_PlayerController.AddGoldQuantity` _asbp_player_controller (`self.Quantity`))
      (`self.K2_DestroyActor`))))

(fn `UserConstructionScript`)