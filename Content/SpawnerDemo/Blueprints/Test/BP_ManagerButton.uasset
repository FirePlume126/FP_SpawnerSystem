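; Floor-plate style test button in the spawner demo that sends entity manager requests when a player-controlled pawn overlaps its trigger.
; ButtonType selects a single request to the named manager, a reset followed by activation, dynamic entity data removal, or a reset of all managers.
; The construction script sets the Chinese label and plate color from ButtonType and RequestType, so each placed instance shows its action.
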(event `self.Trigger.OnComponentBeginOverlap`
  (params (OverlappedComponent :type "PrimitiveComponent Object Reference") (OtherActor :type "Actor Object Reference") (OtherComp :type "PrimitiveComponent Object Reference") (OtherBodyIndex :type Integer) (bFromSweep :type Boolean) (SweepResult :type "HitResult Structure (by ref)"))
  (bind _aspawn (cast `Pawn` OtherActor))
  (if (`Pawn.IsPlayerControlled` _aspawn)
    (switch `/Game/SpawnerDemo/Blueprints/Test/E_ButtonType` (`self.ButtonType`)
      (:`NewEnumerator0`
        (`FPSpawnerFunctionLibrary.TryModifyEntityManagerState` (`self.ManagerName`) (`self.RequestType`)))
      (:`NewEnumerator2`
        (`FPSpawnerFunctionLibrary.TryModifyEntityManagerState` (`self.ManagerName`) "Reset")
        (`FPSpawnerFunctionLibrary.TryModifyEntityManagerState` (`self.ManagerName`) "Activate"))
      (:`NewEnumerator3`
        (`FPSpawnerFunctionLibrary.RemoveDynamicEntityManagerData`))
      (:`NewEnumerator1`
        (`FPSpawnerFunctionLibrary.ResetAllEntityManagers`)))))

(fn `UpdateButton`
  (switch `/Game/SpawnerDemo/Blueprints/Test/E_ButtonType` (`self.ButtonType`)
    (:`NewEnumerator0`
      (`TextRenderComponent.K2_SetText` (`self.Name`) (select `EFPSpawnerEntityManagerRequestType` (`self.RequestType`) :`None` "停 用" :`Activate` "激 活" :`Reset` "重 置" :`Remove` "移 除"))
      (`MeshComponent.SetColorParameterValueOnMaterials` (`self.Plate`) "Color" (select `EFPSpawnerEntityManagerRequestType` (`self.RequestType`) :`None` (struct :`R` 1.0 :`A` 1.0) :`Activate` (struct :`G` 1.0 :`A` 1.0) :`Reset` (struct :`B` 1.0 :`A` 1.0) :`Remove` (struct :`R` 1.0 :`A` 1.0) :!type "LinearColor Structure")))
    (:`NewEnumerator2`
      (`TextRenderComponent.K2_SetText` (`self.Name`) "重置&激活")
      (`MeshComponent.SetColorParameterValueOnMaterials` (`self.Plate`) "Color" (struct :`B` 1.0 :`A` 1.0)))
    (:`NewEnumerator3`
      (`TextRenderComponent.K2_SetText` (`self.Name`) "移除动态 \n实体数据")
      (`MeshComponent.SetColorParameterValueOnMaterials` (`self.Plate`) "Color" (struct :`R` 1.0 :`A` 1.0)))
    (:`NewEnumerator1`
      (`TextRenderComponent.K2_SetText` (`self.Name`) "重置所有")
      (`MeshComponent.SetColorParameterValueOnMaterials` (`self.Plate`) "Color" (struct :`B` 1.0 :`A` 1.0)))))

(fn `UserConstructionScript`
  (`self.UpdateButton`))