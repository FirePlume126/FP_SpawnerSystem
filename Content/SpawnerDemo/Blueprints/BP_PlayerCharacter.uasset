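; Player character for the SpawnerDemo, with Enhanced Input movement, look, jump, sprint, shooting and object placement.
; Sprint and shooting go through server events that set walk speed or run Attack.
; Attack traces from the camera view for an aim point, then spawns BP_Projectile at the hand socket facing it.
; Placing requests a dynamic entity from DA_PlaceObject just in front of the character.
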(event `EnhancedInput|/Game/SpawnerDemo/Input/IA_Move`
  (params (ActionValue :type "Vector2D Structure") (ElapsedSeconds :type "Float (double-precision)") (TriggeredSeconds :type "Float (double-precision)") (InputAction :type "InputAction Object Reference" :default "/Game/SpawnerDemo/Input/IA_Move.IA_Move"))
  (:`Triggered`
    (`self.AddMovementInput` (`self.GetActorRightVector`) ActionValue_X)
    (`self.AddMovementInput` (`self.GetActorForwardVector`) ActionValue_Y)))

(event `EnhancedInput|/Game/SpawnerDemo/Input/IA_Look`
  (params (ActionValue :type "Vector2D Structure") (ElapsedSeconds :type "Float (double-precision)") (TriggeredSeconds :type "Float (double-precision)") (InputAction :type "InputAction Object Reference" :default "/Game/SpawnerDemo/Input/IA_Look.IA_Look"))
  (:`Triggered`
    (`self.AddControllerYawInput` ActionValue_X)
    (`self.AddControllerPitchInput` ActionValue_Y)))

(event `EnhancedInput|/Game/SpawnerDemo/Input/IA_Jump`
  (params (ActionValue :type Boolean) (ElapsedSeconds :type "Float (double-precision)") (TriggeredSeconds :type "Float (double-precision)") (InputAction :type "InputAction Object Reference" :default "/Game/SpawnerDemo/Input/IA_Jump.IA_Jump"))
  (:`Started`
    (`self.Jump`))
  (:`Canceled`
    (`self.StopJumping`)))

(event `EnhancedInput|/Game/SpawnerDemo/Input/IA_Sprint`
  (params (ActionValue :type Boolean) (ElapsedSeconds :type "Float (double-precision)") (TriggeredSeconds :type "Float (double-precision)") (InputAction :type "InputAction Object Reference" :default "/Game/SpawnerDemo/Input/IA_Sprint.IA_Sprint"))
  (:`Started`
    (`self.Server_SetMaxWalkSpeed` 2200.0))
  (:`Completed`
    (`self.Server_SetMaxWalkSpeed` 600.0)))

(event `Server_SetMaxWalkSpeed`
  (params (InSpeed :type "Float (single-precision)"))
  (set `CharacterMovementComponent.MaxWalkSpeed` InSpeed (`self.CharacterMovement`)))

(event `Server_Attack`
  (`self.Attack`))

(event `EnhancedInput|/Game/SpawnerDemo/Input/IA_Shoot`
  (params (ActionValue :type Boolean) (ElapsedSeconds :type "Float (double-precision)") (TriggeredSeconds :type "Float (double-precision)") (InputAction :type "InputAction Object Reference" :default "/Game/SpawnerDemo/Input/IA_Shoot.IA_Shoot"))
  (:`Triggered`
    (`self.Server_Attack`)))

(event `EnhancedInput|/Game/SpawnerDemo/Input/IA_Place`
  (params (ActionValue :type Boolean) (ElapsedSeconds :type "Float (double-precision)") (TriggeredSeconds :type "Float (double-precision)") (InputAction :type "InputAction Object Reference" :default "/Game/SpawnerDemo/Input/IA_Place.IA_Place"))
  (:`Triggered`
    (`FPSpawnerFunctionLibrary.TryCreateDynamicEntityData` "/Game/SpawnerDemo/Data/DA_PlaceObject.DA_PlaceObject" (`self.GetPlaceTransform`) null)))

(fn `Attack`
  (locals (PlayerController :type "PlayerController Object Reference") (TraceStart :type "Vector Structure") (TraceEnd :type "Vector Structure"))
  (bind _tracestart (`local.TraceStart`))
  (bind (_location _rotation) (`Controller.GetPlayerViewPoint` (`local.PlayerController`)))
  (bind _returnvalue (`KismetMathLibrary.GetForwardVector` _rotation))
  (bind _asplayer_controller (cast `PlayerController` (`self.GetController`)))
  (set `local.PlayerController` _asplayer_controller)
  (`|ExecutionSequence`
    (:`then_0`
      (bind _output_get (set `local.TraceStart` (+ _location (* _returnvalue 200.0))))
      (set `local.TraceEnd` (+ _output_get (* _returnvalue 5000.0))))
    (:`then_1`
      (bind (_outhit _returnvalue_2) (`KismetSystemLibrary.LineTraceSingle` (`local.TraceStart`) (`local.TraceEnd`) "TraceTypeQuery1"))
      (set `local.TraceStart` (`SceneComponent.K2_GetComponentLocation` (`self.HandSocket`)))
      (if _returnvalue_2
        (set `local.TraceEnd` (`.ImpactPoint` (`GameplayStatics.BreakHitResult` _outhit)))))
    (:`then_2`
      (`|SpawnActorFromClass` "/Game/SpawnerDemo/Blueprints/Projectile/BP_Projectile.BP_Projectile_C" (`KismetMathLibrary.MakeTransform` _tracestart (`KismetMathLibrary.MakeRotFromX` (- (`local.TraceEnd`) _tracestart))) "AlwaysSpawn" "MultiplyWithRoot" self null))))

(fn `GetPlaceTransform`
  (returns (OutTransform :type "Transform Structure"))
  (return (`KismetMathLibrary.MakeTransform` (+ (`self.K2_GetActorLocation`) (* (`self.GetActorForwardVector`) 100.0) (0.0 0.0 -50.0)) (`self.K2_GetActorRotation`))))

(fn `UserConstructionScript`)