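; StateTree task that makes a bot wander to a random reachable navmesh point around its current location.
; On entering the state, it validates the bot and its controller, picks a point within a fixed radius and runs AI Move To.
; The task finishes as succeeded when the move completes, and as failed if validation, the point search or the move fails.
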(event `self.ReceiveLatentEnterState`
  (params (Transition :type "StateTreeTransitionResult Structure (by ref)"))
  (bind (_randomlocation _returnvalue) (`NavigationSystemV1.K2_GetRandomReachablePointInRadius` (`Actor.K2_GetActorLocation` (`self.Bot`)) 1000.0 null null))
  (`self.Bot`
    (:`then`
      (`/Engine/EditorBlueprintResources/StandardMacros.IsValid` (`Pawn.GetController` (`self.Bot`))
        (:`Is Valid`
          (if _returnvalue
            (`|AIMoveTo` (`self.Bot`) _randomlocation null
              (:`OnSuccess`
                (`self.FinishTask` true))
              (:`OnFail`
                (`self.FinishTask` false)))
            (else
              (`self.FinishTask` false))))
        (:`Is Not Valid`
          (`self.FinishTask` false :!label _label))))
    (:`else`
      (goto _label))))