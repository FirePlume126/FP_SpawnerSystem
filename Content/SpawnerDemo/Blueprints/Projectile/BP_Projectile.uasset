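; BP_Projectile is a red projectile in the spawner demo that reacts to what it hits or overlaps.
; Both hit and overlap events feed HitTarget, which ignores the projectile's owner.
; Actors implementing BPI_Projectile receive an attack message carrying the owner, while other physics-simulating components get an impulse equal to the projectile's velocity.
; The projectile destroys itself only in those two cases.
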(event `self.ReceiveHit`
  (params (MyComp :type "PrimitiveComponent Object Reference") (Other :type "Actor Object Reference") (OtherComp :type "PrimitiveComponent Object Reference") (bSelfMoved :type Boolean) (HitLocation :type "Vector Structure") (HitNormal :type "Vector Structure") (NormalImpulse :type "Vector Structure") (Hit :type "HitResult Structure (by ref)"))
  (`self.HitTarget` Other OtherComp))

(event `self.CollisionComp.OnComponentBeginOverlap`
  (params (OverlappedComponent :type "PrimitiveComponent Object Reference") (OtherActor :type "Actor Object Reference") (OtherComp :type "PrimitiveComponent Object Reference") (OtherBodyIndex :type Integer) (bFromSweep :type Boolean) (SweepResult :type "HitResult Structure (by ref)"))
  (`self.HitTarget` OtherActor OtherComp))

(fn `HitTarget`
  (params (OtherActor :type "Actor Object Reference") (OtherComp :type "PrimitiveComponent Object Reference"))
  (if (!= OtherActor (`self.GetOwner`))
    (if (`KismetSystemLibrary.DoesImplementInterface` OtherActor "/Game/SpawnerDemo/Blueprints/Projectile/BPI_Projectile.BPI_Projectile_C")
      (message `/Game/SpawnerDemo/Blueprints/Projectile/BPI_Projectile.OnAttack` OtherActor (`self.GetOwner`))
      (`self.K2_DestroyActor`)
      (elif (`SceneComponent.IsSimulatingPhysics` OtherComp "None")
        (`PrimitiveComponent.AddImpulseAtLocation` OtherComp (`self.GetVelocity`) (`self.K2_GetActorLocation`) "None")
        (`self.K2_DestroyActor`)))))

(fn `UserConstructionScript`
  (`MeshComponent.SetColorParameterValueOnMaterials` (`self.Sphere`) "Color" (struct :`R` 1.0 :`A` 1.0)))