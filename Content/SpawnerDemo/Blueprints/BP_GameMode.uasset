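; Game mode for the spawner demo that persists spawner state between sessions, with a separate save slot per level.
; On BeginPlay it loads or creates an SG_ServerArchive save object in a slot named after the current level, then applies its stored spawner data.
; On EndPlay it gathers the current spawner data into that archive and writes it back to the same slot.
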(event `self.ReceiveBeginPlay`
  (bind _serverarchive (`self.ServerArchive`))
  (`self.LoadServerArchive`)
  (`/Engine/EditorBlueprintResources/StandardMacros.IsValid` _serverarchive
    (:`Is Valid`
      (`FPSpawnerFunctionLibrary.ApplySpawnerSaveData` (`/Game/SpawnerDemo/SaveGame/SG_ServerArchive.SpawnerSaveData` _serverarchive)))))

(event `self.ReceiveEndPlay`
  (params (EndPlayReason :type "EEndPlayReason Enum" :default "Destroyed"))
  (bind _serverarchive (`self.ServerArchive`))
  (`/Engine/EditorBlueprintResources/StandardMacros.IsValid` (`self.ServerArchive`)
    (:`Is Valid`
      (bind _outsavedata (`FPSpawnerFunctionLibrary.GetSpawnerSaveData`))
      (set `/Game/SpawnerDemo/SaveGame/SG_ServerArchive.SpawnerSaveData` _outsavedata _serverarchive)
      (`GameplayStatics.SaveGameToSlot` _serverarchive (`self.ServerArchiveName`)))))

(fn `LoadServerArchive`
  (bind _returnvalue (`GameplayStatics.GetCurrentLevelName` true))
  (bind _output_get (set `self.ServerArchiveName` (`KismetStringLibrary.Concat_StrStr` "ServerArchive_" _returnvalue)))
  (bind _returnvalue_2 (`GameplayStatics.DoesSaveGameExist` _output_get))
  (if _returnvalue_2
    (bind _returnvalue_3 (`GameplayStatics.LoadGameFromSlot` (`self.ServerArchiveName`)))
    (bind _assg_server_archive (cast `/Game/SpawnerDemo/SaveGame/SG_ServerArchive` _returnvalue_3))
    (set `self.ServerArchive` _assg_server_archive)
    (else
      (bind _returnvalue_4 (`GameplayStatics.CreateSaveGameObject` "/Game/SpawnerDemo/SaveGame/SG_ServerArchive.SG_ServerArchive_C"))
      (set `self.ServerArchive` _returnvalue_4))))

(fn `UserConstructionScript`)